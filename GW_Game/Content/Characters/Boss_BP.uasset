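; Boss tank character that ends the game when destroyed.
; BeginPlay hands the barrel and turret to the aiming component, the track points to the movement component, and links its health bar widget to itself.
; When knocked out, it stops body physics, burns briefly, then explodes with sound, destroys itself and opens the EndMenu level.
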(event `self.ReceiveBeginPlay`
  (`TankAimingComponent.Initialise` (`self.TankAiming`) (`self.TankBarrel`) (`self.Turret`))
  (`TankMovementComponent.Initialise` (`self.TankMovement`) (`self.Left Point`) (`self.Right Point`))
  (`self.InitialiseTankWidget`))

(event `self.TankOutOfAction`
  (bind (_returnvalue_x _returnvalue_y _returnvalue_z) (`KismetMathLibrary.BreakVector` (`self.K2_GetActorLocation`)))
  (bind (_returnvalue_x_2 _returnvalue_y_2 _returnvalue_z_2) (`KismetMathLibrary.BreakVector` (`self.K2_GetActorLocation`)))
  (`PrimitiveComponent.SetSimulatePhysics` (`self.Body`) false)
  (bind _returnvalue (`GameplayStatics.SpawnEmitterAtLocation` "/Game/Characters/MyFire.MyFire" (`KismetMathLibrary.MakeVector` _returnvalue_x_2 _returnvalue_y_2 (+ _returnvalue_z_2 200.0))))
  (`KismetSystemLibrary.Delay` 1.0)
  (`ActorComponent.K2_DestroyComponent` _returnvalue)
  (`GameplayStatics.SpawnEmitterAtLocation` "/Game/Projectile/ImpactBlast.ImpactBlast" (`KismetMathLibrary.MakeVector` _returnvalue_x _returnvalue_y (+ _returnvalue_z 100.0)))
  (`GameplayStatics.PlaySoundAtLocation` "/Game/Projectile/Explosion01.Explosion01" (`self.K2_GetActorLocation`))
  (`self.K2_DestroyActor`)
  (`GameplayStatics.OpenLevel` "EndMenu"))

(fn `InitialiseTankWidget`
  (bind _ashealth_bar (cast `/Game/UI/HealthBar` (`WidgetComponent.GetUserWidgetObject` (`self.Widget`))))
  (set `/Game/UI/HealthBar.MyTank` self _ashealth_bar))

(fn `UserConstructionScript`)